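; Firun handles the game's win and defeat sequences for the character passed to its events, and caches the first Flamy actor on BeginPlay.
; YouDied locks play, reveals the death display, then after a delay destroys Firun and opens the Procedural_P level.
; YouWin hides the exit arrow, swaps music, mutes flames and shows a flipbook cinematic.
; It times a delay from the flipbook's length, then stops it and sets GameFinished.
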(event `self.ReceiveBeginPlay`
  (`|ExecutionSequence`
    (:`then_0`
      (bind _outactors (`GameplayStatics.GetAllActorsOfClass` "/Game/Blueprints/Flamy.Flamy_C"))
      (if (> (`KismetArrayLibrary.Array_Length` _outactors) 0)
        (set `self.Flamy` (`|GetArrayItem` _outactors))))))

(event `YouDied`
  (params (Char :type "/Game/Blueprints/Flamy Object Reference"))
  ;[1 1 1] Logic defaite
  (`/Game/Blueprints/Flamy.CantPlay` Char)
  (`SceneComponent.SetHiddenInGame` (`/Game/Blueprints/Flamy.Die` Char) false true)
  (`KismetSystemLibrary.Delay` 5.0)
  (`self.K2_DestroyActor`)
  (`GameplayStatics.OpenLevel` "Procedural_P"))

(event `YouWin`
  (params (Char :type "/Game/Blueprints/Flamy Object Reference"))
  (bind _cinematique (`/Game/Blueprints/Flamy.Cinematique` Char))
  (bind _music (`/Game/Blueprints/Flamy.Music` Char))
  ;[1 1 1] Logic win
  (`SceneComponent.SetVisibility` (`/Game/Blueprints/Flamy.ExitArrow` Char) false false)
  (`AudioComponent.SetVolumeMultiplier` _music (`/Game/Blueprints/Flamy.MusicVolume` Char))
  (`AudioComponent.SetSound` _music "/Game/Audio/bensound-hey_Cue.bensound-hey_Cue")
  (`AudioComponent.SetVolumeMultiplier` (`/Game/Blueprints/Flamy.Flames` Char) 0.0)
  (`SceneComponent.SetHiddenInGame` _cinematique false true)
  (`PaperFlipbookComponent.SetFlipbook` _cinematique "/Game/Textures/Cinematique/Fin/cinematique2.cinematique2")
  (`KismetSystemLibrary.Delay` (* (/ 1.0 (`PaperFlipbookComponent.GetPlayRate` _cinematique)) (/ (`KismetMathLibrary.Conv_IntToDouble` (`PaperFlipbookComponent.GetFlipbookLengthInFrames` _cinematique)) (`PaperFlipbook.FramesPerSecond` (`PaperFlipbookComponent.GetFlipbook` _cinematique)))))
  (`PaperFlipbookComponent.Stop` _cinematique)
  (set `self.GameFinished` true))

(fn `UserConstructionScript`)